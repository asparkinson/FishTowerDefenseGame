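; GM_Level2 is the Level 2 game mode, running wave progression and the win state.
; On BeginPlay it shows the GameHUD and caches the first BP_Grid, exposed through GetGrid.
; StartWave increments the wave counter, sets PlayerWin once it exceeds four, maps waves one to three to matching difficulties, then starts the SpawnerLV2 spawner.
; Difficulty stays unchanged after wave three, and spawning is still triggered after a win.
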(event Custom|StartWave
  (Math|Integer|IncrementInt (Variables|Default|GetCurrentWaveNumber)
    (:%20%20
      (CallFunction|WinCondition)
      (CallFunction|DifficultySelect)
      (bind _spawner (CallFunction|GetSpawners))
      (Default|StartWave _spawner (Variables|Default|GetDifficulty)))))

(event Custom|DifficultySelect
  (if (== (Variables|Default|GetCurrentWaveNumber) 1)
    (Variables|Default|SetDifficulty 1)
    (elif (== (Variables|Default|GetCurrentWaveNumber) 2)
      (Variables|Default|SetDifficulty 2)
      (elif (== (Variables|Default|GetCurrentWaveNumber) 3)
        (Variables|Default|SetDifficulty 3)))))

(event Custom|WinCondition
  (if (> (Variables|Default|GetCurrentWaveNumber) 4)
    (Variables|Default|SetPlayerWin true)))

(event EventBeginPlay
  (bind _returnvalue (UserInterface|CreateWidget "/Game/MyContent/Blueprints/GameHUD.GameHUD_C"))
  (UserInterface|Viewport|AddtoViewport _returnvalue 0)
  (bind _outactors (Actor|GetAllActorsOfClass "/Game/MyContent/Blueprints/BP_Grid.BP_Grid_C"))
  (Variables|Default|SetGrid (Utilities|Array|Get(acopy) _outactors)))

(fn ConstructionScript)

(fn GetSpawners
  (bind _returnvalue (Actor|GetActorOfClass "/Game/MyContent/Blueprints/SpawnerLV2.SpawnerLV2_C"))
  (bind _output_get (Variables|Default|SetSpawner_2 _returnvalue))
  (return 0 _output_get))

(fn GetGrid
  (return (Variables|Default|GetGrid)))