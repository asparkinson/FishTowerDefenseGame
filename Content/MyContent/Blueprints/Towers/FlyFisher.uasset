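; FlyFisher is a tower Blueprint that supplies the fisher's sprite-based catch animation.
; Its PlaySpriteMontage event swaps the sprite component to the catch-state sprite and material, then restores the idle pair after a brief Delay, acting as a two-frame montage.
; Tick only forwards to the parent, BeginPlay is disabled, and nothing in this file triggers the montage.
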(event EventBeginPlay
  (|CallParentFunction) ; This node is disabled and will not be called.\nDrag off pins to build functionality.
)

(event Collision|EventActorBeginOverlap
  (params (OtherActor :type Actor%20Object%20Reference)))

(event EventTick
  (params (DeltaSeconds :type Float%20%28single-precision%29))
  (|CallParentFunction DeltaSeconds))

(event EventPlaySpriteMontage
  (bind _new_piskel_1_png__1__sprite (Variables|Default|GetNew_Piskel-1_png__1__Sprite))
  (bind _new_piskel_1_png__1__sprite_2 (Variables|Default|GetNew_Piskel-1_png__1__Sprite))
  (Rendering|Components|Sprite|SetSprite _new_piskel_1_png__1__sprite "/Game/MyContent/Sprites/fisherCatchState_Sprite.fisherCatchState_Sprite")
  (Rendering|Material|SetMaterial _new_piskel_1_png__1__sprite 0 "/Game/MyContent/Assets/Fishermen/fisherCatchState_Mat.fisherCatchState_Mat")
  (Utilities|FlowControl|Delay 0.2)
  (Rendering|Components|Sprite|SetSprite _new_piskel_1_png__1__sprite_2 "/Game/MyContent/Sprites/FlyFisher_Sprite.FlyFisher_Sprite")
  (Rendering|Material|SetMaterial _new_piskel_1_png__1__sprite_2 0 "/Game/MyContent/Assets/Fishermen/fisher_Mat.fisher_Mat"))

(fn ConstructionScript
  (|CallParentFunction))