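; Base shore fisherman tower for a tower defense game that turns toward fish in range and damages them.
; A targeting sphere queues overlapping fish, targets the first and drops the oldest entry whenever an overlap ends.
; While a target is present, Tick interpolates rotation toward it and calls the catch, with a Delay pacing attacks.
; Each rod fires an offset forward sphere trace, skipping the gamemode's ignore list, and damages hit actors.
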(event OnComponentBeginOverlap(FishTargettingSphere)
  (params (OverlappedComponent :type Primitive%20Component%20Object%20Reference) (OtherActor :type Actor%20Object%20Reference) (OtherComp :type Primitive%20Component%20Object%20Reference) (OtherBodyIndex :type Integer) (bFromSweep :type Boolean) (SweepResult :type Hit%20Result%20Structure%20%28by%20ref%29))
  (bind _targetsarray (Variables|Default|GetTargetsArray))
  (bind _output (Utilities|Array|Get(acopy) _targetsarray))
  (bind _asfish_base (Utilities|Casting|CastToFishBase OtherActor))
  (Variables|Default|SetTargetInRange true)
  (Utilities|Array|Add _targetsarray _asfish_base)
  (if (not (== _output (Variables|Default|GetCurrentTarget)))
    (Variables|Default|SetCurrentTarget _output)))

(event OnComponentEndOverlap(FishTargettingSphere)
  (params (OverlappedComponent :type Primitive%20Component%20Object%20Reference) (OtherActor :type Actor%20Object%20Reference) (OtherComp :type Primitive%20Component%20Object%20Reference) (OtherBodyIndex :type Integer))
  (bind _targetsarray (Variables|Default|GetTargetsArray))
  (Utilities|Array|RemoveIndex _targetsarray)
  (if (Utilities|Array|IsNotEmpty _targetsarray)
    (Variables|Default|SetCurrentTarget (Utilities|Array|Get(acopy) _targetsarray))
    (else
      (Variables|Default|SetTargetInRange false))))

(event Custom|LookAtFish
  (Utilities|IsValid (Variables|Default|GetCurrentTarget)
    (:Is%20Valid
      (Transformation|SetActorRotation (Math|Interpolation|RInterpTo (Transformation|GetActorRotation) (Math|Rotator|FindLookatRotation (Transformation|GetActorLocation) (Transformation|GetActorLocation (Variables|Default|GetCurrentTarget))) (Utilities|Time|GetWorldDeltaSeconds) 2e+01) true))))

(event Custom|AttemptCatch
  (bind _returnvalue (Transformation|GetActorLocation))
  (Utilities|FlowControl|Delay (Variables|Default|GetTowerAttackDelay))
  (Variables|Default|SetStartLocation (Math|Vector|MakeVector (+ (.x _returnvalue) 2e+01) (.y _returnvalue) (.z _returnvalue)))
  (for _index (range 1 (Variables|Default|GetRodsNum))
    (bind _outhit (Collision|SphereTraceByChannel (Variables|Default|GetStartLocation) (+ (Variables|Default|GetStartLocation) (* (Transformation|GetActorForwardVector) 65.0)) 15.0 "TraceTypeQuery1" false (Variables|/Game/MyContent/Blueprints/TowerDefenseGamemode.TowerDefenseGamemode_C|GetActorsFishermanIgnore (Variables|Default|GetTower%20Defense%20Gamemode)) "ForDuration" true "(R=1.000000,G=0.000000,B=0.000000,A=1.000000)" "(R=0.000000,G=1.000000,B=0.000000,A=1.000000)" 0.2))
    (Variables|Default|SetStartLocation (Math|Vector|MakeVector (- (.x (Variables|Default|GetStartLocation)) 1e+01) (.y (Variables|Default|GetStartLocation)) (.z (Variables|Default|GetStartLocation))))
    (if (Utilities|IsValid (.HitActor (Collision|BreakHitResult _outhit)))
      (Game|Damage|ApplyDamage (.HitActor (Collision|BreakHitResult _outhit)) (Variables|Default|GetTowerDamage) 0 0))))

(event EventTick
  (params (DeltaSeconds :type Float%20%28single-precision%29))
  (if (Variables|Default|GetTargetInRange)
    (CallFunction|LookatFish)
    (CallFunction|AttemptCatch)))

(event EventBeginPlay
  (bind _astower_defense_gamemode (Utilities|Casting|CastToTowerDefenseGamemode (Game|GetGameMode)))
  (bind _output_get (Variables|Default|SetTower%20Defense%20Gamemode _astower_defense_gamemode))
  (Utilities|Array|Add (Variables|/Game/MyContent/Blueprints/TowerDefenseGamemode.TowerDefenseGamemode_C|GetActorsFishermanIgnore _output_get) self))

(fn ConstructionScript)