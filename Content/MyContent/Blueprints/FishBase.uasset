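; FishBase is a fish actor that travels along a spline path and can be killed by damage.
; On BeginPlay it finds a FishSpline actor in the level and starts a timeline.
; The timeline alpha is lerped over the spline length to set world location and rotation on each update.
; Damage reduces Health, and the actor destroys itself once Health drops below zero.
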(event Custom|Death
  (Actor|DestroyActor))

(event Custom|Start%20Moving
  (bind _alpha (Timeline|Timeline Play)
    (:Update
      (Transformation|SetActorLocationAndRotation (.location (Spline|GetTransformatDistanceAlongSpline (Variables|/Game/MyContent/Blueprints/FishSpline.FishSpline_C|GetSpline (Variables|Default|GetPath)) (Math|Float|Lerp 0.0 (Spline|GetSplineLength (Variables|/Game/MyContent/Blueprints/FishSpline.FishSpline_C|GetSpline (Variables|Default|GetPath))) _alpha) "World" false)) (.rotation (Spline|GetTransformatDistanceAlongSpline (Variables|/Game/MyContent/Blueprints/FishSpline.FishSpline_C|GetSpline (Variables|Default|GetPath)) (Math|Float|Lerp 0.0 (Spline|GetSplineLength (Variables|/Game/MyContent/Blueprints/FishSpline.FishSpline_C|GetSpline (Variables|Default|GetPath))) _alpha) "World" false))))))

(event EventBeginPlay
  (bind _returnvalue (Actor|GetActorOfClass "/Game/MyContent/Blueprints/FishSpline.FishSpline_C"))
  (Variables|Default|SetPath _returnvalue)
  (CallFunction|StartMoving))

(event Collision|EventActorBeginOverlap
  (params (OtherActor :type Actor%20Object%20Reference)))

(event EventTick
  (params (DeltaSeconds :type Float%20%28single-precision%29)))

(event Game|Damage|EventAnyDamage
  (params (Damage :type Float%20%28single-precision%29) (DamageType :type Damage%20Type%20Object%20Reference) (InstigatedBy :type Controller%20Object%20Reference) (DamageCauser :type Actor%20Object%20Reference))
  (if (> (Variables|Default|GetHealth) 0.0)
    (bind _output_get (Variables|Default|SetHealth (- (Variables|Default|GetHealth) Damage)))
    (if (< _output_get 0.0)
      (CallFunction|Death))))

(fn ConstructionScript)