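; Enemy spawner actor that spawns enemies from a class queue at its own transform.
; A looping sub-second timer started on BeginPlay calls SpawnEnemy, which spawns the first queued class or prints "False" when the queue is empty.
; AddEnemyToQueue appends a class and spawns immediately if no FishBase overlaps its Sphere.
; The queue removal node is disconnected, so the first entry is never dequeued and spawns repeatedly.
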(event Custom|TryToSpawn
  (CallFunction|SpawnEnemy))

(event EventBeginPlay
  (Utilities|Time|SetTimerbyEvent (delegate Custom|TryToSpawn) 0.75 true))

(fn ConstructionScript)

(fn SpawnEnemy
  (if (Utilities|Array|IsValidIndex (Variables|Default|GetEnemyQueue))
    (Game|SpawnActorfromClass (Utilities|Array|Get(acopy) (Variables|Default|GetEnemyQueue)) (Transformation|GetActorTransform) "Undefined" "MultiplyWithRoot" 0 0)
    (return true)
    (else
      (Development|PrintString "False")
      (return false))))

(fn AddEnemytoQueue
  (params (EnemyClass :type Fish%20Base%20Class%20Reference%20%28by%20ref%29))
  (Utilities|Array|Add (Variables|Default|GetEnemyQueue) EnemyClass)
  (if (not (Utilities|Array|IsValidIndex (Collision|GetOverlappingActors (Variables|Default|GetSphere) "/Game/MyContent/Blueprints/FishBase.FishBase_C" :!class /Script/Engine.PrimitiveComponent)))
    (CallFunction|SpawnEnemy)))