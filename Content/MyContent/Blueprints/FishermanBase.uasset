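; Base tower defense fisherman that turns toward a fish in range and damages what is in front of it.
; Its targeting sphere locks the first overlap through a DoOnce, which any end overlap resets.
; Tick interpolates rotation toward the target and calls AttemptCatch, whose Delay paces short debug-drawn sphere traces that apply damage, skipping actors on the gamemode's ignore list.
; An array-based targeting system is unfinished and unused.
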(event OnComponentBeginOverlap(FishTargettingSphere)
  (params (OverlappedComponent :type Primitive%20Component%20Object%20Reference) (OtherActor :type Actor%20Object%20Reference) (OtherComp :type Primitive%20Component%20Object%20Reference) (OtherBodyIndex :type Integer) (bFromSweep :type Boolean) (SweepResult :type Hit%20Result%20Structure%20%28by%20ref%29))
  (Utilities|FlowControl|DoOnce false
    (:Completed
      (bind _asfish_base (Utilities|Casting|CastToFishBase OtherActor))
      (Variables|Default|SetTargetInRange true)
      (Variables|Default|SetCurrentTarget _asfish_base))))

(event OnComponentEndOverlap(FishTargettingSphere)
  (params (OverlappedComponent :type Primitive%20Component%20Object%20Reference) (OtherActor :type Actor%20Object%20Reference) (OtherComp :type Primitive%20Component%20Object%20Reference) (OtherBodyIndex :type Integer))
  (Variables|Default|SetCurrentTarget OtherActor)
  (Variables|Default|SetTargetInRange false)
  (Utilities|FlowControl|DoOnce false) ; enters at Reset
)

(event Custom|LookAtFish
  (Transformation|SetActorRotation (Math|Interpolation|RInterpTo (Transformation|GetActorRotation) (Math|Rotator|FindLookatRotation (Transformation|GetActorLocation) (Transformation|GetActorLocation (Variables|Default|GetCurrentTarget))) (Utilities|Time|GetWorldDeltaSeconds) 2e+01) true))

(event Custom|AttemptCatch
  (Utilities|FlowControl|Delay 0.5)
  (bind _outhit (Collision|SphereTraceByChannel (Transformation|GetActorLocation) (+ (Transformation|GetActorLocation) (* (Transformation|GetActorForwardVector) 65.0)) 1e+01 "TraceTypeQuery1" false (Variables|Default|GetActors%20to%20Ignore) "ForDuration" true "(R=1.000000,G=0.000000,B=0.000000,A=1.000000)" "(R=0.000000,G=1.000000,B=0.000000,A=1.000000)" 0.2))
  (if (Utilities|IsValid (.HitActor (Collision|BreakHitResult _outhit)))
    (Game|Damage|ApplyDamage (.HitActor (Collision|BreakHitResult _outhit)) 11.0 0 0)))

(event Custom|MakeCurrentTarget
  ;[0.15 0.15 0.15 0.5] WIP New Target System
  (if (Utilities|Array|IsValidIndex (Variables|Default|GetTargetsArray))
    (Variables|Default|SetCurrentTarget 0)))

(event EventTick
  (params (DeltaSeconds :type Float%20%28single-precision%29))
  (if (Variables|Default|GetTargetInRange)
    (CallFunction|LookatFish)
    (CallFunction|AttemptCatch)))

(event EventBeginPlay
  (bind _astower_defense_gamemode (Utilities|Casting|CastToTowerDefenseGamemode (Game|GetGameMode)))
  (bind _output_get (Variables|Default|SetTower%20Defense%20Gamemode _astower_defense_gamemode))
  (bind _output_get_2 (Variables|Default|SetActors%20to%20Ignore (Variables|/Game/MyContent/Blueprints/TowerDefenseGamemode.TowerDefenseGamemode_C|GetActorsFishermanIgnore _output_get)))
  (Utilities|Array|Add _output_get_2 self))

(fn ConstructionScript)