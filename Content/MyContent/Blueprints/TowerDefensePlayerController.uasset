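; Player controller for a fisherman-themed tower defense game that handles touch placement of towers and creates the game HUD.
; PlaceTower stores the chosen tower class and arms placement mode.
; A tap on a TowerPlacement-tagged actor spawns it snapped through BPCGrid at fixed height, then calls the HUD's BuyTower.
; With nothing selected, tapping a FlyFisher opens its upgrades widget; a DoOnce reset on release limits each touch to one action.
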(event Custom|PlaceTower
  (params (TowerToPlace :type Actor%20Class%20Reference))
  (Variables|Default|SetFishermanActor TowerToPlace)
  (Variables|Default|SetTowerSelected true))

(event EventBeginPlay
  (Variables|Default|SetbShowMouseCursor true)
  (bind _returnvalue (UserInterface|CreateWidget "/Game/MyContent/Blueprints/GameHUD.GameHUD_C"))
  (bind _output_get (Variables|Default|SetGameHUD _returnvalue))
  (UserInterface|Viewport|AddtoViewport _output_get 0))

(event Input|TouchEvents|Touch1
  (params (Key :type Key%20Structure :default "None"))
  (bind _hitresult (Class|PlayerController|GetHitResultUnderFingerbyChannel "Touch1" "TraceTypeQuery1" true))
  (bind _bpc_grid (Variables|Default|GetBPC_Grid))
  (bind (_bblockinghit _binitialoverlap _time _distance _location _impactpoint _normal _impactnormal _physmat _hitactor) (Collision|BreakHitResult _hitresult))
  (bind _locationongrid (Default|GetGridLocation _bpc_grid _location))
  ;[0.15 0.15 0.15 0.5] Touch Tower Placement
  (:Pressed
    (Utilities|FlowControl|DoOnce false :!label _label
      (:Completed
        (if (Variables|Default|GetTowerSelected)
          (if (Actor|ActorHasTag _hitactor "TowerPlacement")
            (Game|SpawnActorfromClass (Variables|Default|GetFishermanActor) (Math|Transform|MakeTransform (Math|Vector|MakeVector (.x _locationongrid) (.y _locationongrid) 5.0) "0, 0, 0" "1.000000,1.000000,1.000000") "Undefined" "MultiplyWithRoot" 0 0)
            (Variables|Default|SetTowerSelected false)
            (Variables|Default|SetStopPlacingButtonVisible false)
            (Default|BuyTower (Variables|Default|GetGameHUD)))
          (else
            (Utilities|FlowControl|Sequence
              (:then_0
                (if (== (Utilities|Array|Get(acopy) (Variables|/Script/Engine.Actor|GetTags _hitactor)) "FlyFisher")
                  (bind _returnvalue (UserInterface|CreateWidget "/Game/MyContent/Blueprints/UpgradesUI/FlyFisherUpgrades.FlyFisherUpgrades_C"))
                  (UserInterface|Viewport|AddtoViewport _returnvalue 0)))))))))
  (:Released
    (goto _label Reset)))

(fn ConstructionScript)