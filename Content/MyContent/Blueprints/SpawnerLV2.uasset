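; Level 2 wave spawner that spawns fish at its own transform in waves of three difficulty tiers.
; StartWave applies a tier preset for fish class, count, spawn delay and play rate, then spawns through a custom ForLoopWithDelay macro.
; Tick compares EnemiesKilled, which is not incremented here, to the wave size, resetting it and raising WaveEnded until the next non-matching tick.
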(event Custom|EasyDifficulty
  (Variables|Default|SetEnemiesToSpawn 4)
  (Variables|Default|SetFishPlayRate 1.2)
  (Variables|Default|SetDelayBetweenSpawn 1.5)
  (Variables|Default|SetFishToSpawnClass "/Game/MyContent/Blueprints/Enemies/SheepsHead.SheepsHead_C"))

(event Custom|MedDifficulty
  (Variables|Default|SetEnemiesToSpawn 7)
  (Variables|Default|SetFishPlayRate 1.6)
  (Variables|Default|SetDelayBetweenSpawn 0.75)
  (Variables|Default|SetFishToSpawnClass "/Game/MyContent/Blueprints/Enemies/CatFish.CatFish_C"))

(event Custom|HardDifficulty
  (Variables|Default|SetEnemiesToSpawn 10)
  (Variables|Default|SetFishPlayRate 2.2)
  (Variables|Default|SetDelayBetweenSpawn 0.2)
  (Variables|Default|SetFishToSpawnClass "/Game/MyContent/Blueprints/Enemies/Shark.Shark_C"))

(event Custom|StartWave
  (params (SetDifficulty :type Integer))
  (bind _output_get (Variables|Default|SetDifficulty SetDifficulty))
  (switch int _output_get
    (:1
      (CallFunction|EasyDifficulty))
    (:2
      (CallFunction|MedDifficulty))
    (:3
      (CallFunction|HardDifficulty)))
  (Utilities|ForLoopwithDelay 0 (Variables|Default|GetEnemiesToSpawn) (Variables|Default|GetDelayBetweenSpawn)
    (:Loop%20Body
      (Game|SpawnActorfromClass (Variables|Default|GetFishToSpawnClass) (Transformation|GetActorTransform) "Undefined" "MultiplyWithRoot" 0 0))))

(event EventBeginPlay)

(event EventTick
  (params (DeltaSeconds :type Float%20%28single-precision%29))
  (if (== (Variables|Default|GetEnemiesKilled) (Variables|Default|GetEnemiesToSpawn))
    (Variables|Default|SetWaveEnded true)
    (Variables|Default|SetEnemiesKilled 0)
    (else
      (Variables|Default|SetWaveEnded false))))

(fn ConstructionScript)