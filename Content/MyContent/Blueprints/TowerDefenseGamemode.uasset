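; Tower defense game mode that creates the game HUD at BeginPlay and tracks wave progression, difficulty and the win state.
; StartWave increments the wave number, flags a player win once it passes a fixed limit, then maps the first waves to rising difficulty levels.
; It then passes the difficulty to the EnemySpawner found by GetActorOfClass, even when the win flag is set.
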(event Custom|StartWave
  (Math|Integer|IncrementInt (Variables|Default|GetCurrentWaveNumber)
    (:%20%20
      (CallFunction|WinCondition)
      (CallFunction|DifficultySelect)
      (bind _spawner (CallFunction|GetSpawners))
      (Default|StartWave _spawner (Variables|Default|GetDifficulty)))))

(event Custom|DifficultySelect
  (if (== (Variables|Default|GetCurrentWaveNumber) 1)
    (Variables|Default|SetDifficulty 1)
    (elif (== (Variables|Default|GetCurrentWaveNumber) 2)
      (Variables|Default|SetDifficulty 2)
      (elif (== (Variables|Default|GetCurrentWaveNumber) 3)
        (Variables|Default|SetDifficulty 3)))))

(event Custom|WinCondition
  (if (> (Variables|Default|GetCurrentWaveNumber) 4)
    (Variables|Default|SetPlayerWin true)))

(event EventBeginPlay
  (bind _returnvalue (UserInterface|CreateWidget "/Game/MyContent/Blueprints/GameHUD.GameHUD_C"))
  (UserInterface|Viewport|AddtoViewport _returnvalue 0))

(fn ConstructionScript)

(fn GetSpawners
  (bind _returnvalue (Actor|GetActorOfClass "/Game/MyContent/Blueprints/EnemySpawner.EnemySpawner_C"))
  (bind _output_get (Variables|Default|SetSpawner _returnvalue))
  (return _output_get))